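; BP_Enemy_Shooter_Blue is a shooter enemy that fires on BP_Monster_Basic pawns it sees.
; PawnSensing sightings are filtered by a cast, and the actor snaps its rotation to face the seen pawn.
; If CanAttack is set, it spawns a BP_SecondProjectile at SpawnProjectileLocation, then uses a flag and Delay cooldown to limit the fire rate.
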(event OnSeePawn(PawnSensing)
  (params (Pawn :type Pawn%20Object%20Reference))
  (bind _asbp_monster_basic (Utilities|Casting|CastToBP_Monster_Basic Pawn))
  (Transformation|SetActorRotation (Math|Rotator|FindRelativeLookatRotation (Math|Conversions|ToTransform(Vector) (Transformation|GetActorLocation)) (Transformation|GetActorLocation _asbp_monster_basic)))
  (if (Variables|Default|GetCanAttack)
    (Game|SpawnActorfromClass "/Game/BluePrints/BP_SecondProjectile.BP_SecondProjectile_C" (Transformation|GetWorldTransform (Variables|Default|GetSpawnProjectileLocation)) "Undefined" "MultiplyWithRoot" 0 0)
    (Variables|Default|SetCanAttack false)
    (Utilities|FlowControl|Delay 3.0)
    (Variables|Default|SetCanAttack true)))

(event EventBeginPlay)

(event Collision|EventActorBeginOverlap
  (params (OtherActor :type Actor%20Object%20Reference)))

(event EventTick
  (params (DeltaSeconds :type Float%20%28single-precision%29)))

(fn ConstructionScript)