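; Game mode for what its name suggests is a basic monster level, setting up the HUD, music and input when play begins.
; On BeginPlay it removes the LevelInfo widget, adds a BP_UI widget to the viewport, switches to game-only input and hides the mouse cursor.
; Music playback goes through BP_MyGameInstance, which is asked to play the LovelyPlanet track.
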(event EventBeginPlay
  (bind _returnvalue (Game|GetPlayerController 0))
  (Widget|RemovefromParent (Variables|Default|GetLevelInfo))
  (Input|SetInputModeGameOnly (Game|GetPlayerController 0) false)
  (bind _returnvalue_2 (UserInterface|CreateWidget "/Game/BluePrints/UI/BP_UI.BP_UI_C"))
  (UserInterface|Viewport|AddtoViewport _returnvalue_2 0)
  (bind _asbp_my_game_instance (Utilities|Casting|CastToBP_MyGameInstance (Game|GetGameInstance)))
  (Default|PlayMusic _asbp_my_game_instance "/Game/Audios/LovelyPlanet.LovelyPlanet")
  (Input|SetInputModeGameOnly _returnvalue false)
  (Variables|/Script/Engine.PlayerController|SetbShowMouseCursor _returnvalue false))

(fn ConstructionScript)