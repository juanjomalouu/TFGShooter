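; BP_Monster_Basic, despite its name, holds only per-level best-time save logic in this graph.
; BeginPlay loads HighTime from a BP_SaveGameHS slot, or creates the save and seeds the level's entry with its level number.
; SetRecord saves CurrentTime when it is lower than the stored score, recreating the save if missing.
; The HighScores index is parsed from two characters at a fixed position in the level name.
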(event Custom|Set%20Record
  (bind _currenttime (Variables|Default|GetCurrentTime))
  (bind _returnvalue (Game|GetCurrentLevelName true))
  (bind _asbp_save_game_hs (Utilities|Casting|CastToBP_SaveGameHS (Variables|Default|GetSaverSubClass)))
  (Math|Float|CompareFloat _currenttime (Utilities|Array|Get(acopy) (Variables|/Game/BluePrints/Game/BP_SaveGameHS.BP_SaveGameHS_C|GetHighScores _asbp_save_game_hs) (Math|Float|Truncate (Math|Conversions|ToFloat(Integer) (Utilities|String|GetSubstring _returnvalue 8 2))))
    (:<
      (Variables|Default|SetHighTime _currenttime)
      (bind _returnvalue_2 (SaveGame|DoesSaveGameExist (Variables|Default|GetSlot%20Name)))
      (if _returnvalue_2
        (bind _returnvalue_3 (SaveGame|LoadGamefromSlot (Variables|Default|GetSlot%20Name)))
        (bind _output_get (Variables|Default|SetSaverSubClass _returnvalue_3))
        (bind _asbp_save_game_hs_2 (Utilities|Casting|CastToBP_SaveGameHS _output_get))
        (bind _output_get_2 (Variables|/Game/BluePrints/Game/BP_SaveGameHS.BP_SaveGameHS_C|SetHighScores _asbp_save_game_hs_2 (Variables|/Game/BluePrints/Game/BP_SaveGameHS.BP_SaveGameHS_C|GetHighScores _asbp_save_game_hs_2)))
        (Utilities|Array|SetArrayElem _output_get_2 (Math|Float|Truncate (Math|Conversions|ToFloat(Integer) (Utilities|String|GetSubstring _returnvalue 8 2))) _currenttime)
        (SaveGame|SaveGametoSlot (Variables|Default|GetSaverSubClass) (Variables|Default|GetSlot%20Name))
        (else
          (bind _returnvalue_4 (SaveGame|CreateSaveGameObject "/Game/BluePrints/Game/BP_SaveGameHS.BP_SaveGameHS_C"))
          (SaveGame|SaveGametoSlot _returnvalue_4 (Variables|Default|GetSlot%20Name))
          (bind _output_get_3 (Variables|Default|SetSaverSubClass _returnvalue_4))
          (bind _asbp_save_game_hs_3 (Utilities|Casting|CastToBP_SaveGameHS _output_get_3))
          (bind _output_get_4 (Variables|/Game/BluePrints/Game/BP_SaveGameHS.BP_SaveGameHS_C|SetHighScores _asbp_save_game_hs_3 (Variables|/Game/BluePrints/Game/BP_SaveGameHS.BP_SaveGameHS_C|GetHighScores _asbp_save_game_hs_3)))
          (Utilities|Array|SetArrayElem _output_get_4 (Math|Float|Truncate (Math|Conversions|ToFloat(Integer) (Utilities|String|GetSubstring _returnvalue 8 2))) _currenttime)
          (SaveGame|SaveGametoSlot (Variables|Default|GetSaverSubClass) (Variables|Default|GetSlot%20Name)))))))

(event EventBeginPlay
  (bind _slot_name (Variables|Default|GetSlot%20Name))
  (bind _returnvalue (SaveGame|DoesSaveGameExist _slot_name))
  (if _returnvalue
    (bind _returnvalue_2 (SaveGame|LoadGamefromSlot _slot_name))
    (bind _output_get (Variables|Default|SetSaverSubClass _returnvalue_2))
    (bind _asbp_save_game_hs (Utilities|Casting|CastToBP_SaveGameHS _output_get))
    (bind _returnvalue_3 (Game|GetCurrentLevelName true))
    (Variables|Default|SetHighTime (Utilities|Array|Get(acopy) (Variables|/Game/BluePrints/Game/BP_SaveGameHS.BP_SaveGameHS_C|GetHighScores _asbp_save_game_hs) (Math|Float|Truncate (Math|Conversions|ToFloat(Integer) (Utilities|String|GetSubstring _returnvalue_3 8 2)))))
    (else
      (bind _returnvalue_4 (SaveGame|CreateSaveGameObject "/Game/BluePrints/Game/BP_SaveGameHS.BP_SaveGameHS_C"))
      (SaveGame|SaveGametoSlot _returnvalue_4 (Variables|Default|GetSlot%20Name))
      (bind _output_get_2 (Variables|Default|SetSaverSubClass _returnvalue_4))
      (bind _asbp_save_game_hs_2 (Utilities|Casting|CastToBP_SaveGameHS _output_get_2))
      (bind _output_get_3 (Variables|/Game/BluePrints/Game/BP_SaveGameHS.BP_SaveGameHS_C|SetHighScores _asbp_save_game_hs_2 (Variables|/Game/BluePrints/Game/BP_SaveGameHS.BP_SaveGameHS_C|GetHighScores _asbp_save_game_hs_2)))
      (bind _returnvalue_5 (Game|GetCurrentLevelName true))
      (Utilities|Array|SetArrayElem _output_get_3 (Math|Float|Truncate (Math|Conversions|ToFloat(Integer) (Utilities|String|GetSubstring _returnvalue_5 8 2))) (Math|Conversions|ToFloat(Integer) (Utilities|String|GetSubstring _returnvalue_5 8 2)))
      (SaveGame|SaveGametoSlot (Variables|Default|GetSaverSubClass) (Variables|Default|GetSlot%20Name)))))

(fn ConstructionScript)